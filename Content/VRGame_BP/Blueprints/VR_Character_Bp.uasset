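; VR player pawn for robot arena melee combat, where the player punches enemies with motion controllers.
; Each tick it moves the actor to follow the headset, measures each hand's per-frame horizontal displacement as velocity, and checks for defeat.
; Hand overlaps above a speed threshold play a punch sound and damage EnemyCharacter_BP.
; It also handles head/body damage, flags loss on the player controller, toggles HP widgets and records grab input.
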(event OnComponentBeginOverlap(HitCollison_L)
  (params (OverlappedComponent :type Primitive%20Component%20Object%20Reference) (OtherActor :type Actor%20Object%20Reference) (OtherComp :type Primitive%20Component%20Object%20Reference) (OtherBodyIndex :type Integer) (bFromSweep :type Boolean) (SweepResult :type Hit%20Result%20Structure%20%28by%20ref%29))
  ;[1 1 1] Hiting system
  (if (not (== (Pawn|GetControlledPawn (Game|GetPlayerController 0)) OtherActor))
    (if (> (Variables|Default|GetLeftControllerVelocity) 5.0)
      (CallFunction|HandleHitEvent OtherActor OtherComp "Left")
      (CallFunction|PlayHitSound (Transformation|GetWorldLocation OtherComp)))))

(event OnComponentBeginOverlap(HitCollison_R)
  (params (OverlappedComponent :type Primitive%20Component%20Object%20Reference) (OtherActor :type Actor%20Object%20Reference) (OtherComp :type Primitive%20Component%20Object%20Reference) (OtherBodyIndex :type Integer) (bFromSweep :type Boolean) (SweepResult :type Hit%20Result%20Structure%20%28by%20ref%29))
  ;[1 1 1] Hiting system
  (if (not (== (Pawn|GetControlledPawn (Game|GetPlayerController 0)) OtherActor))
    (if (> (Variables|Default|GetRightControllerVelocity) 5.0)
      (CallFunction|HandleHitEvent OtherActor OtherComp "Right")
      (CallFunction|PlayHitSound (Transformation|GetWorldLocation OtherComp)))))

(event EventTick
  (params (DeltaSeconds :type Float%20%28single-precision%29))
  ;[1 1 1] Event Tick
  (CallFunction|AdjustHMD)
  (CallFunction|GetLeftMCVelocity (Transformation|GetWorldLocation (Variables|Default|GetMotionController_L)))
  (CallFunction|GetRightMCVelocity (Transformation|GetWorldLocation (Variables|Default|GetMotionController_R)))
  (CallFunction|CheckLost))

(event EventBeginPlay
  ;[1 1 1] Begin Play
  (CallFunction|InitHMD)
  (CallFunction|InitHandCollison))

(event Input|ActionEvents|InputActionRightHandGrab
  (params (Key :type Key%20Structure))
  ;[1 1 1] Handle Input For Grab
  (:Pressed
    (Variables|Default|SetRightHandGrab true))
  (:Released
    (Variables|Default|SetRightHandGrab false)))

(event Input|ActionEvents|InputActionLeftHandGrab
  (params (Key :type Key%20Structure))
  ;[1 1 1] Handle Input For Grab
  (:Pressed
    (Variables|Default|SetLeftHandGrab true))
  (:Released
    (Variables|Default|SetLeftHandGrab false)))

(event Input|ActionEvents|InputActionUIOnLeft
  (params (Key :type Key%20Structure))
  ;[1 1 1] Enable UI Input Handle
  (:Pressed
    (CallFunction|DetermineUIVisibility)))

(event Input|ActionEvents|InputActionUIOnRight
  (params (Key :type Key%20Structure))
  ;[1 1 1] Enable UI Input Handle
  (:Pressed
    (CallFunction|DetermineUIVisibility)))

(fn ConstructionScript)

(fn InitHMD
  (Variables|/Script/Engine.CameraComponent|SetbUsePawnControlRotation (Variables|Default|GetFollowCamera) false)
  (Transformation|AddRelativeLocation (Variables|Default|GetVROrigin) (Math|Vector|MakeVector 0.0 0.0 (* (Components|Capsule|GetScaledCapsuleHalfHeight (Variables|Default|GetCapsuleComponent)) -1.0)) false false)
  (Class|HeadMountedDisplayFunctionLibrary|ResetOrientationandPosition 0.0 "Orientation"))

(fn AdjustHMD
  (bind (_devicerotation _deviceposition) (Class|HeadMountedDisplayFunctionLibrary|GetOrientationandPosition))
  (bind _vrorigin (Variables|Default|GetVROrigin))
  (Components|Capsule|SetCapsuleHalfHeight (Variables|Default|GetCapsuleComponent) (+ 0.0 5.0) true)
  (if (Class|HeadMountedDisplayFunctionLibrary|HasValidTrackingPosition)
    (LocalVariables|SetOriginTargetTransform (Transformation|GetWorldTransform _vrorigin))
    (LocalVariables|SetActorTargetTransform (Math|Transform|MakeTransform (+ (Math|Vector|NegateVector (Math|Vector|MakeVector 3e+01 3e+01 (.Z (Math|Vector|BreakVector (.DevicePosition (Class|HeadMountedDisplayFunctionLibrary|GetOrientationandPosition)))))) (Math|Vector|MakeVector 0.0 0.0 (+ (Components|Capsule|GetScaledCapsuleHalfHeight (Variables|Default|GetCapsuleComponent)) 0.0)) (.Location (Math|Transform|BreakTransform (Math|Transform|ComposeTransforms (Math|Transform|MakeTransform _deviceposition _devicerotation) (LocalVariables|GetOriginTargetTransform))))) (Math|Rotator|MakeRotator 0.0 0.0 (.Yaw (Math|Rotator|BreakRotator (.Rotation (Math|Transform|BreakTransform (Math|Transform|ComposeTransforms (Math|Transform|MakeTransform _deviceposition _devicerotation) (LocalVariables|GetOriginTargetTransform)))))))))
    (Transformation|SetRelativeTransform _vrorigin (Class|KismetMathLibrary|ConvertTransformtoRelative (LocalVariables|GetActorTargetTransform) (LocalVariables|GetOriginTargetTransform)) false false)
    (Transformation|SetActorTransform (LocalVariables|GetActorTargetTransform) true)))

(fn GetLeftMCVelocity
  (params (ActualState :type Vector))
  (if (Math|Vector|Equal(Vector) (Variables|Default|GetPreviousStateL) "0, 0, 0" 0.0)
    (Variables|Default|SetPreviousStateL ActualState)
    (return)
    (else
      (Variables|Default|SetLeftControllerVelocity (Math|Vector|VectorLengthXY (- ActualState (Variables|Default|GetPreviousStateL))))
      (Variables|Default|SetPreviousStateL ActualState)
      (return))))

(fn GetRightMCVelocity
  (params (ActualState :type Vector))
  (if (Math|Vector|Equal(Vector) (Variables|Default|GetPreviousStateR) "0, 0, 0" 0.0001)
    (Variables|Default|SetPreviousStateR ActualState)
    (return)
    (else
      (Variables|Default|SetRightControllerVelocity (Math|Vector|VectorLengthXY (- ActualState (Variables|Default|GetPreviousStateR))))
      (Variables|Default|SetPreviousStateR ActualState)
      (return))))

(fn AdjustMasstoVelocity
  (return))

(fn HandleHitEvent
  (params (WhoGotHit :type Actor%20Object%20Reference) (WhereGotHit :type Primitive%20Component%20Object%20Reference) (WhichHand :type Text))
  (bind _asenemy_character_bp (Utilities|Casting|CastToEnemyCharacter_BP WhoGotHit)
    (:then
      (Default|GetDamage _asenemy_character_bp WhereGotHit WhichHand)
      (return))
    (:CastFailed
      (return))))

(fn PlayHitSound
  (params (HitLocation :type Vector))
  (Audio|PlaySoundatLocation "/Game/VRGame_BP/Blueprints/Audio/PunchSoundCue.PunchSoundCue" HitLocation)
  (return))

(fn InitHandCollison
  (Variables|/Script/Engine.PrimitiveComponent|SetbGenerateOverlapEvents (Variables|Default|GetHitCollison_R) true)
  (Variables|/Script/Engine.PrimitiveComponent|SetbGenerateOverlapEvents (Variables|Default|GetHitCollison_L) true)
  (return))

(fn DetermineUIVisibility
  (bind _enemyhpwidget (Variables|Default|GetEnemyHPWidget))
  (bind _playerhpwidget (Variables|Default|GetPlayerHPWidget))
  (bind _output_get (Variables|Default|SetisVisible? (not (Variables|Default|GetisVisible?))))
  (if _output_get
    (Audio|PlaySound2D "/Game/VRGame_BP/Blueprints/Audio/UIOnSound.UIOnSound")
    (Rendering|SetVisibility _enemyhpwidget true false)
    (Rendering|SetVisibility _playerhpwidget true false)
    (Variables|Default|SetisVisible? true)
    (else
      (Rendering|SetVisibility _enemyhpwidget false false)
      (Rendering|SetVisibility _playerhpwidget false false)
      (Variables|Default|SetisVisible? false)))
  (return))

(fn ApplyDamage
  (params (WhereGotHit? :type Primitive%20Component%20Object%20Reference))
  (if (== (Variables|Default|GetHeadCollison) WhereGotHit?)
    (Variables|Default|SetHealth (- (Variables|Default|GetHealth) 1e+01))
    (return)
    (elif (== WhereGotHit? (Variables|Default|GetBodyCollison))
      (Variables|Default|SetHealth (- (Variables|Default|GetHealth) 5.0))
      (return)
      (else
        (return)))))

(fn CheckLost
  (if (<= (Variables|Default|GetHealth) 0.0)
    (bind _asrobot_arena_player_controller (Utilities|Casting|CastToRobotArenaPlayerController (Game|GetPlayerController 0)))
    (Variables|/Game/VRGame_BP/Blueprints/RobotArenaPlayerController.RobotArenaPlayerController_C|SetLost? _asrobot_arena_player_controller true)
    (return)
    (else
      (return))))