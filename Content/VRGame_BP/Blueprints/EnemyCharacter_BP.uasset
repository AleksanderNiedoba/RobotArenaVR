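; VR melee enemy character that reacts physically to hits and ragdolls at zero health.
; On BeginPlay it enables physical animation below a configurable bone and caches the player's VR_Character.
; Head collision overlaps subtract damage scaled by the hitting hand's controller velocity, plus a bonus when that hand is grabbing.
; Tick prints health and, at zero or below, clears the animation drive strengths and simulates physics on the whole mesh.
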(event OnComponentBeginOverlap(HeadCollison)
  (params (OverlappedComponent :type Primitive%20Component%20Object%20Reference) (OtherActor :type Actor%20Object%20Reference) (OtherComp :type Primitive%20Component%20Object%20Reference) (OtherBodyIndex :type Integer) (bFromSweep :type Boolean) (SweepResult :type Hit%20Result%20Structure%20%28by%20ref%29))
  (bind _vr_characterreference (Variables|Default|GetVR_CharacterReference))
  (bind _damage (CallFunction|CalculateDamage (Variables|/Game/VRGame_BP/Blueprints/VR_Character.VR_Character_C|GetRightHandHit _vr_characterreference) (Variables|/Game/VRGame_BP/Blueprints/VR_Character.VR_Character_C|GetLeftHandHit _vr_characterreference)))
  (Variables|Default|SetHealth (- (Variables|Default|GetHealth) _damage)))

(event EventBeginPlay
  (CallFunction|SetPhysicsProperties)
  (CallFunction|GetVRCharactrReference))

(event EventTick
  (params (DeltaSeconds :type Float%20%28single-precision%29))
  (bind _health (Variables|Default|GetHealth))
  (Development|PrintString (Utilities|String|ToString(Float) _health))
  (if (<= _health 0.0)
    (CallFunction|TurnOffPhysics)
    (Physics|SetSimulatePhysics (Variables|Character|GetMesh) true)))

(fn ConstructionScript)

(fn SetPhysicsProperties
  (bind _physicalanimation (Variables|Default|GetPhysicalAnimation))
  (bind _bonename (Variables|Default|GetBoneName))
  (Class|PhysicalAnimationComponent|SetSkeletalMeshComponent _physicalanimation (Variables|Character|GetMesh))
  (Class|PhysicalAnimationComponent|ApplyPhysicalAnimationSettingsBelow _physicalanimation _bonename (Utilities|Struct|MakePhysicalAnimationData false 1e+03 2e+02 1e+03 2e+02) false)
  (Class|SkeletalMeshComponent|SetAllBodiesBelowSimulatePhysics (Variables|Character|GetMesh) _bonename true false)
  (return))

(fn GetVRCharactrReference
  (bind _asvr_character (Utilities|Casting|CastToVR_Character (Pawn|GetControlledPawn (Game|GetPlayerController 0))))
  (Variables|Default|SetVR_CharacterReference _asvr_character)
  (return))

(fn CalculateDamage
  (params (Right :type Boolean) (Left :type Boolean))
  (bind _vr_characterreference (Variables|Default|GetVR_CharacterReference))
  (if Right
    (bind _output_get (LocalVariables|SetLocalDamage (* 1e+01 (Variables|/Game/VRGame_BP/Blueprints/VR_Character.VR_Character_C|GetRightControllerVelocity _vr_characterreference))))
    (if (Variables|/Game/VRGame_BP/Blueprints/VR_Character.VR_Character_C|GetRightHandGrab _vr_characterreference)
      (bind _output_get_2 (LocalVariables|SetLocalDamage (+ _output_get 1e+01)))
      (return _output_get_2)
      (else
        (return (LocalVariables|GetLocalDamage))))
    (elif Left
      (bind _output_get_3 (LocalVariables|SetLocalDamage (* 1e+01 (Variables|/Game/VRGame_BP/Blueprints/VR_Character.VR_Character_C|GetLeftControllerVelocity _vr_characterreference))))
      (if (Variables|/Game/VRGame_BP/Blueprints/VR_Character.VR_Character_C|GetLeftHandGrab _vr_characterreference)
        (bind _output_get_4 (LocalVariables|SetLocalDamage (+ _output_get_3 1e+01)))
        (return _output_get_4))
      (else
        (return (LocalVariables|GetLocalDamage))))))

(fn TurnOffPhysics
  (bind _physicalanimation (Variables|Default|GetPhysicalAnimation))
  (bind _bonename (Variables|Default|GetBoneName))
  (Class|PhysicalAnimationComponent|SetSkeletalMeshComponent _physicalanimation (Variables|Character|GetMesh))
  (Class|PhysicalAnimationComponent|ApplyPhysicalAnimationSettingsBelow _physicalanimation _bonename (Utilities|Struct|MakePhysicalAnimationData false 0.0) false)
  (Class|SkeletalMeshComponent|SetAllBodiesBelowSimulatePhysics (Variables|Character|GetMesh) _bonename true false)
  (return))